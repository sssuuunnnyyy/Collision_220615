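; BP_TimeLineMove is an actor that slides a Sphere back and forth along relative X using a timeline scaled by EndPoint.
; On finish, the timeline flips IsMoveRight and re-enters the branch to play or reverse, creating a ping-pong loop.
; BeginPlay binds to the ThirdPersonCharacter's F-key dispatcher, apparently driving the pressed-state function that starts or stops movement.
; A separate Play function offers the same start/stop control.
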(event `PlayEvent`
  ;[1 1 1] 상태에 따른 실행라인 방향 처리
  (if (`self.IsMoveRight`) :!label _label
    (bind (_direction _value) (`Timeline|타임라인_0` :`NewTime` 2.5 :!label _label_2)
      (:`Update`
        ;[1 1 1] 이동
        (`SceneComponent.K2_SetRelativeLocation` (`self.Sphere`) (`KismetMathLibrary.MakeVector` (* _value (`self.EndPoint`))) false false))
      (:`Finished`
        ;[1 1 1] 방향 바꾸기
        (set `self.IsMoveRight` (not (`self.IsMoveRight`)))
        (goto _label)))
    (else
      (goto _label_2 :!via `Reverse`))))

(event `StopEvent`
  (goto _label_2 :!via `Stop`))

(event `self.ReceiveBeginPlay`
  (bind _asthird_person_character (cast `/Game/ThirdPersonBP/Blueprints/ThirdPersonCharacter` (`GameplayStatics.GetPlayerCharacter` 0)))
  (add `/Game/ThirdPersonBP/Blueprints/ThirdPersonCharacter.EventDispatcher_F_Key` _asthird_person_character (`|CreateDelegate` :!event `BP_TimeLineMove_AutoGenFunc`)))

(fn `BP_TimeLineMove_AutoGenFunc`
  (params (IsPressed :type Boolean))
  (if IsPressed
    (`self.PlayEvent`)
    (else
      (`self.StopEvent`))))

(fn `Play`
  (params (IsPlay :type Boolean))
  (returns (Result :type Boolean))
  (if IsPlay
    (`self.PlayEvent`)
    (else
      (`self.StopEvent`)))
  (return true))

(fn `UserConstructionScript`)