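; Actor Blueprint that moves its Cube component up and down between a relative height of zero and EndPoint while playback is on.
; Tick applies a fixed per-frame Z offset without delta-time scaling or sweep, so speed depends on frame rate.
; IsMoveRight holds the vertical direction despite its name and flips at each limit.
; The Play function sets IsPlay to start or pause the motion.
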(event `self.ReceiveTick`
  (params (DeltaSeconds :type "Float (single-precision)"))
  (bind _cube (`self.Cube`))
  (bind (_relativelocation_x _relativelocation_y _relativelocation_z) (`KismetMathLibrary.BreakVector` (`SceneComponent.RelativeLocation` _cube)))
  (bind (_relativelocation_x_2 _relativelocation_y_2 _relativelocation_z_2) (`KismetMathLibrary.BreakVector` (`SceneComponent.RelativeLocation` _cube)))
  (if (`self.isPlay`)
    (if (`self.IsMoveRight`)
      (`SceneComponent.K2_AddRelativeLocation` _cube (0.0 0.0 5.0) false false)
      (if (>= _relativelocation_z_2 (`self.EndPoint`))
        (set `self.IsMoveRight` false))
      (else
        (`SceneComponent.K2_AddRelativeLocation` (`self.Cube`) (0.0 0.0 -5.0) false false)
        (if (< _relativelocation_z 0.0)
          (set `self.IsMoveRight` true))))))

(fn `Play`
  (params (isPlay :type Boolean))
  (set `self.isPlay` isPlay))

(fn `UserConstructionScript`)